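; Test Blueprint that connects to a MIDI input device and shows its incoming events as on-screen debug text.
; On BeginPlay it scans MIDI devices for an input whose ID matches MIDIControllerIndex, creates a controller for it and binds to OnMIDIEvent.
; The event handler prints type, note and velocity under a shared key, so each message replaces the previous one.
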(event `self.ReceiveBeginPlay`
  (bind _outmididevices (`MIDIDeviceManager.FindMIDIDevices`))
  (for _array_element _outmididevices
    (bind (_deviceid _devicename _bcanreceivefrom) (break `FoundMIDIDevice` _array_element))
    (if _bcanreceivefrom
      (if (== (`self.MIDIControllerIndex`) _deviceid)
        (`KismetSystemLibrary.PrintString` _devicename true true (struct :`R` 0.018872 :`G` 1.0 :`B` 0.077227 :`A` 1.0) 30.0)
        (bind _returnvalue (`MIDIDeviceManager.CreateMIDIDeviceController` _deviceid))
        (bind _output_get (set `self.MIDIControl` _returnvalue))
        (add `MIDIDeviceController.OnMIDIEvent` _output_get (`|CreateDelegate` :!event `onMIDIevent`)))))
  (`KismetSystemLibrary.PrintString` "BOUCLE TERMINÉE" true true (struct :`R` 0.47909 :`G` 1.0 :`B` 0.432292 :`A` 1.0) 30.0))

(event `onMIDIevent`
  (params (MIDIDeviceController :type "MIDIDeviceController Object Reference") (Timestamp :type Integer) (EventType :type "EMIDIEventType Enum" :default "Unknown") (Channel :type Integer) (ControlID :type Integer) (Velocity :type Integer) (RawEventType :type Integer))
  (`KismetSystemLibrary.PrintString` (`KismetTextLibrary.Conv_TextToString` (`|FormatText` "MIDI EVENT TYPE {event} MIDI Note {note} VELOCITE {velocite}" (`|GetEnumeratorNameAsString` EventType) ControlID Velocity)) true true (struct :`R` 0.022159 :`G` 1.0 :`B` 0.005638 :`A` 1.0) 2.0 "MIDI"))

(fn `UserConstructionScript`)