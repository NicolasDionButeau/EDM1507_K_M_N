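; MIDI manager Blueprint that turns input from a hardware controller into MetaSound playback.
; BeginPlay finds the device matching MIDIControllerIndex, binds a MIDI event handler and starts a persistent low-pass filter MetaSound.
; EventonMIDI spawns a synth sound per selected pad note, passing the note number, and maps a knob to normalized filter cutoff.
; CustomEvent plays another sound for different notes; reverb and drive setters are unconnected.
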(event `self.ReceiveBeginPlay`
  (bind _outmididevices (`MIDIDeviceManager.FindMIDIDevices`))
  (for _array_element _outmididevices
    (bind (_deviceid _devicename _bcanreceivefrom) (break `FoundMIDIDevice` _array_element))
    (if _bcanreceivefrom
      (if (== (`self.MIDI_controller_index`) _deviceid)
        (`KismetSystemLibrary.PrintString` _devicename true true (struct :`G` 0.66 :`B` 1.0 :`A` 1.0) 30.0)
        (bind _returnvalue (`MIDIDeviceManager.CreateMIDIDeviceController` _deviceid))
        (bind _output_get (set `self.MIDIcontrol` _returnvalue))
        (add `MIDIDeviceController.OnMIDIEvent` _output_get (`|CreateDelegate` :!event `EventonMIDI`)))))
  (`KismetSystemLibrary.PrintString` "BOUCLE TERMINÉE" true true (struct :`G` 0.66 :`B` 1.0 :`A` 1.0) 30.0)
  ; lpf
  (bind _returnvalue_2 (`GameplayStatics.CreateSound2D` "/Game/metasounds/MSS_LPF_K2.MSS_LPF_K2" 1.0 1.0 0.0 null))
  (set `self.lpf metasound` _returnvalue_2)
  (`AudioComponent.Play` _returnvalue_2 0.0))

(event `EventonMIDI`
  (params (MIDIDeviceController :type "MIDIDeviceController Object Reference") (Timestamp :type Integer) (EventType :type "EMIDIEventType Enum" :default "Unknown") (Channel :type Integer) (ControlID :type Integer) (Velocity :type Integer) (RawEventType :type Integer))
  ; Aynth 01
  ;; Imprimer à l'écran
  (`KismetSystemLibrary.PrintString` (`KismetTextLibrary.Conv_TextToString` (`|FormatText` "MIDI EVENT TYPE {event} MIDI note{note} VELOCITE {velocite} CHANNEL {chan}" (`|GetEnumeratorNameAsString` EventType) ControlID Velocity Channel)) true true (struct :`R` 0.168419 :`G` 1.0 :`B` 0.247111 :`A` 1.0) 2.0 "MIDI")
  (switch `EMIDIEventType` EventType
    (:`NoteOn`
      (switch `string` (`KismetStringLibrary.Conv_IntToString` ControlID)
        (:`53`
          _)
        (:`55`
          _)
        (:`57`
          _)
        (:`59`
          _)
        (:`60`
          _)
        (:`62`
          _)
        (:`64`
          _)
        (:`65`
          _))
      ;;[0.8438 0.1802 0.7544 0.5] Notes sur le pad
      (bind _returnvalue (`GameplayStatics.CreateSound2D` "/Game/metasounds/MSS_synth_K2.MSS_synth_K2" 1.0 1.0 0.0 null))
      (`AudioParameterControllerInterface.SetFloatParameter` _returnvalue "MIDI note" (`KismetMathLibrary.Conv_IntToDouble` ControlID))
      (`AudioComponent.Play` _returnvalue 0.0))
    (:`ControlChange`
      ;; filter sur le MIDI controller
      (switch `string` (`KismetStringLibrary.Conv_IntToString` ControlID)
        (:`114`
          ;;; Cutoff
          (`AudioParameterControllerInterface.SetFloatParameter` (`self.lpf metasound`) "Cutoff Frequency" (/ (`KismetMathLibrary.Conv_IntToDouble` Velocity) 127.0)))))))

(event `CustomEvent`
  (params (MIDIDeviceController :type "MIDIDeviceController Object Reference") (Timestamp :type Integer) (EventType :type "EMIDIEventType Enum" :default "Unknown") (Channel :type Integer) (ControlID :type Integer) (Velocity :type Integer) (RawEventType :type Integer))
  ; Aynth 01
  ;; Imprimer à l'écran
  (`KismetSystemLibrary.PrintString` (`KismetTextLibrary.Conv_TextToString` (`|FormatText` "MIDI EVENT TYPE {event} MIDI note{note} VELOCITE {velocite} CHANNEL {chan}" (`|GetEnumeratorNameAsString` EventType) ControlID Velocity Channel)) true true (struct :`R` 0.168419 :`G` 1.0 :`B` 0.247111 :`A` 1.0) 2.0 "MIDI")
  (switch `EMIDIEventType` EventType
    (:`NoteOn`
      (switch `string` (`KismetStringLibrary.Conv_IntToString` ControlID)
        (:`25`
          _)
        (:`27`
          _)
        (:`30`
          _)
        (:`54`
          _))
      ;;[0.8438 0.1802 0.7544 0.5] Notes sur le pad
      (bind _returnvalue (`GameplayStatics.CreateSound2D` "/Game/metasounds/MSS_YEEE1.MSS_YEEE1" 1.0 1.0 0.0 null))
      (`AudioParameterControllerInterface.SetFloatParameter` _returnvalue "MIDI note" (`KismetMathLibrary.Conv_IntToDouble` ControlID))
      (`AudioComponent.Play` _returnvalue 0.0))
    (:`ControlChange`
      ;; filter sur le MIDI controller
      (switch `string` (`KismetStringLibrary.Conv_IntToString` ControlID)))))

(fn `UserConstructionScript`)